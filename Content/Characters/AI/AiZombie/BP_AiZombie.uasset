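; Zombie AI character that chases the player once pawn sensing spots a pawn and attacks on arrival.
; Seeing a pawn sets a flag and starts an AI MoveTo toward the player; Tick halts movement while that flag is unset.
; A successful move triggers Attack, gated by DoOnce, which disables movement during a random attack montage.
; Fixed damage lands on the player after a short delay, without a range recheck.
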(event `self.PawnSensing.OnSeePawn`
  (params (Pawn :type "Pawn Object Reference"))
  (set `self.IsSeeingPlayer?` true)
  (`self.Follow Player`))

(event `Follow Player`
  (set `self.CanAttack?` true)
  (if (`self.IsSeeingPlayer?`)
    (`|AIMoveTo` self (0.0 0.0 0.0) (`GameplayStatics.GetPlayerCharacter` 0)
      (:`OnSuccess`
        (if (`self.CanAttack?`)
          (set `self.CanAttack?` false)
          (bind _returnvalue (`self.PlayAnimMontage` null))
          (`KismetSystemLibrary.Delay` _returnvalue)
          (set `self.CanAttack?` true)
          (`self.Attack`))))
    (else
      (set `self.IsSeeingPlayer?` false))))

(event `self.ReceiveTick`
  (params (DeltaSeconds :type "Float (single-precision)"))
  (if (not (`self.IsSeeingPlayer?`))
    (`MovementComponent.StopMovementImmediately` (`self.CharacterMovement`))))

(event `Attack`
  (bind _attackanims (`self.AttackAnims`))
  (`/Engine/EditorBlueprintResources/StandardMacros.DoOnce` false :!label _label
    (:`Completed`
      (`CharacterMovementComponent.DisableMovement` (`self.CharacterMovement`))
      (`|ExecutionSequence`
        (:`then_0`
          (`|PlayMontage` (`self.Mesh`) (`|GetArrayItem` _attackanims (`KismetMathLibrary.RandomInteger` (`KismetArrayLibrary.Array_Length` _attackanims)))
            (:`OnCompleted`
              _)
            (:`OnInterrupted`
              (`KismetSystemLibrary.Delay` 1.0)))
          (`CharacterMovementComponent.SetMovementMode` (`self.CharacterMovement`) "MOVE_Walking" 0)
          (goto _label :!via `Reset`))
        (:`then_1`
          (`KismetSystemLibrary.Delay` 0.75)
          (`GameplayStatics.ApplyDamage` (`GameplayStatics.GetPlayerCharacter` 0) 5.0 null self))))))

(fn `UserConstructionScript`)