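; BP_BreakingFlashlight is an interactable, single-use trigger actor that breaks the player's flashlight.
; Interacting with it or overlapping its Box runs the same check on player character 0 through message calls for flashlight possession and broken state.
; A working flashlight gets a break message after the actor calls destroy on itself, while an already broken one only prints a debug string.
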(event `self.OnInteract`
  (params (InteractingPlayer :type "Character Object Reference"))
  (bind _return (message `/Game/Blueprints/Interfaces/BPI_Flashlight.CheckIfPlayerHasFlashlihght?` (`GameplayStatics.GetPlayerCharacter` 0) :!label _label))
  (if _return
    (bind _return_2 (message `/Game/Blueprints/Interfaces/BPI_Flashlight.CheckIfFlashLightBroken` (`GameplayStatics.GetPlayerCharacter` 0)))
    (if _return_2
      (`KismetSystemLibrary.PrintString` "Flashlight already broken")
      (else
        (`self.K2_DestroyActor`)
        (message `/Game/Blueprints/Interfaces/BPI_Flashlight.BreakFlashlight` (`GameplayStatics.GetPlayerCharacter` 0))))))

(event `self.Box.OnComponentBeginOverlap`
  (params (OverlappedComponent :type "PrimitiveComponent Object Reference") (OtherActor :type "Actor Object Reference") (OtherComp :type "PrimitiveComponent Object Reference") (OtherBodyIndex :type Integer) (bFromSweep :type Boolean) (SweepResult :type "HitResult Structure (by ref)"))
  (goto _label))

(fn `IsInteractable`
  (returns (Interactable :type Boolean))
  (return true))

(fn `UserConstructionScript`)