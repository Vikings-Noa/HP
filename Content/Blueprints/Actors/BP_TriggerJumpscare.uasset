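; BP_TriggerJumpscare is a trigger actor that fires a jumpscare on the player character.
; On BeginPlay it caches the player pawn as an HP_Character reference.
; The first overlap of its Box component calls JUMPSCARE on that character, and the first end overlap calls JUMPSCAREOFF after a one-second delay.
; DoOnce gates make each side single-use, and neither overlap checks which actor triggered it.
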(event `self.ReceiveBeginPlay`
  (bind _ashp_character (cast `/Game/HP_Character` (`GameplayStatics.GetPlayerCharacter` 0)))
  (set `self.Char Ref` _ashp_character))

(event `self.Box.OnComponentBeginOverlap`
  (params (OverlappedComponent :type "PrimitiveComponent Object Reference") (OtherActor :type "Actor Object Reference") (OtherComp :type "PrimitiveComponent Object Reference") (OtherBodyIndex :type Integer) (bFromSweep :type Boolean) (SweepResult :type "HitResult Structure (by ref)"))
  (`/Engine/EditorBlueprintResources/StandardMacros.DoOnce` false
    (:`Completed`
      (`/Game/HP_Character.JUMPSCARE` (`self.Char Ref`)))))

(event `self.Box.OnComponentEndOverlap`
  (params (OverlappedComponent :type "PrimitiveComponent Object Reference") (OtherActor :type "Actor Object Reference") (OtherComp :type "PrimitiveComponent Object Reference") (OtherBodyIndex :type Integer))
  (`/Engine/EditorBlueprintResources/StandardMacros.DoOnce` false
    (:`Completed`
      (`KismetSystemLibrary.Delay` 1.0)
      (`/Game/HP_Character.JUMPSCAREOFF` (`self.Char Ref`)))))

(fn `UserConstructionScript`)