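; BP_Battery is an interactable pickup that repairs the player's broken flashlight.
; On interact, it queries the player character through message calls for whether a flashlight is held and broken.
; If so, it destroys itself and tells the player to repair it; a working flashlight only prints an on-screen notice.
; Without a flashlight, interacting does nothing.
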(event `/Game/Blueprints/Interfaces/BPI_Interact.OnInteract`
  (params (InteractingPlayer :type "Character Object Reference"))
  (bind _return (message `/Game/Blueprints/Interfaces/BPI_Flashlight.CheckIfPlayerHasFlashlihght?` (`GameplayStatics.GetPlayerCharacter` 0)))
  (if _return
    (bind _return_2 (message `/Game/Blueprints/Interfaces/BPI_Flashlight.CheckIfFlashLightBroken` (`GameplayStatics.GetPlayerCharacter` 0)))
    (if _return_2
      (`self.K2_DestroyActor`)
      (message `/Game/Blueprints/Interfaces/BPI_Flashlight.RepairFlashlight` (`GameplayStatics.GetPlayerCharacter` 0))
      (else
        (`KismetSystemLibrary.PrintString` "Your Flashlight Already Has A Battery!")))))

(fn `IsInteractable`
  (returns (Interactable :type Boolean))
  (return true))

(fn `UserConstructionScript`)