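; Interactable electricity lever switch that toggles its HasElectricity flag, which starts as true.
; OnInteract alternates forward and reverse lever montages on the skeletal mesh, whose physics is disabled at BeginPlay, guarded by IsAnimating.
; Switching off updates state and releases the guard as soon as the montage starts, while switching on waits for completion.
; UpdateSwitchesAndLight is an empty stub.
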(event `self.ReceiveBeginPlay`
  (`SkeletalMeshComponent.SetAllBodiesSimulatePhysics` (`self. switch skeletal`) false)
  (`PrimitiveComponent.SetSimulatePhysics` (`self. switch skeletal`) false))

(event `/Game/Blueprints/Interfaces/BPI_Interact.OnInteract`
  (params (InteractingPlayer :type "Character Object Reference"))
  (if (not (`self.isAnimating?`))
    (if (`self.isAnimationPlayed?`)
      (set `self.isAnimating?` true)
      (`|PlayMontage` (`self. switch skeletal`) "/Game/Props/ElectricitySwitch/Lever_Switch_Anim_MontageReverse.Lever_Switch_Anim_MontageReverse" -1.0 1.0
        (:`OnCompleted`
          (set `self.isAnimationPlayed?` false)
          (set `self.hasElectricity?` true)))
      (else
        (set `self.isAnimating?` true)
        (`|PlayMontage` (`self. switch skeletal`) "/Game/Props/ElectricitySwitch/Lever_Switch_Anim_Montage.Lever_Switch_Anim_Montage" 1.0 -1.0 "None" false
          (:`then`
            (set `self.isAnimationPlayed?` true)
            (set `self.hasElectricity?` false)))))
    (set `self.isAnimating?` false)))

(fn `IsInteractable`
  (returns (Interactable :type Boolean))
  (return true))

(fn `UpdateSwitchesAndLight`)

(fn `UserConstructionScript`
  (set `self.hasElectricity?` true))