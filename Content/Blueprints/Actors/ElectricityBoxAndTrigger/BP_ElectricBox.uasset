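; BP_ElectricBox is an interactable electricity box whose door swings open and closed when the player interacts.
; OnInteract toggles the open state, plays the matching 2D sound, and plays or reverses a timeline that drives the door pivot's yaw.
; An animating flag ignores interactions until the timeline finishes, and IsInteractable always returns true.
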(event `/Game/Blueprints/Interfaces/BPI_Interact.OnInteract`
  (params (InteractingPlayer :type "Character Object Reference"))
  (bind _doorpivot (`self.DoorPivot`))
  (bind (_relativerotation_roll _relativerotation_pitch) (`KismetMathLibrary.BreakRotator` (`SceneComponent.RelativeRotation` _doorpivot)))
  (if (`self.isDoorAnimating?`)
    _
    (elif (not (`self.isDoorOpen?`))
      (set `self.isDoorAnimating?` true)
      (set `self.isDoorOpen?` true)
      (`GameplayStatics.PlaySound2D` "/Game/Audio/OpeningBox.OpeningBox" 1.0 1.0 0.0 null null)
      (bind (_direction _alpha) (`Timeline|Open/Colse ElectricityBoxDoor` :!label _label)
        (:`Update`
          (`SceneComponent.K2_SetRelativeRotation` _doorpivot (`KismetMathLibrary.MakeRotator` _relativerotation_roll _relativerotation_pitch _alpha) false false))
        (:`Finished`
          (set `self.isDoorAnimating?` false)))
      (else
        (set `self.isDoorAnimating?` true)
        (set `self.isDoorOpen?` false)
        (`GameplayStatics.PlaySound2D` "/Game/Audio/ClosingBox.ClosingBox" 1.0 1.0 0.0 null null)
        (goto _label :!via `Reverse`)))))

(fn `IsInteractable`
  (returns (Interactable :type Boolean))
  (return true))

(fn `UserConstructionScript`)