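; An interactable light switch that toggles a linked electric light, provided its linked electricity switch has power.
; Interacting turns the light on or off based on its current state, or prints a no-electricity message when power is missing.
; Tick polls the electricity switch and turns the light off on every frame without power.
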(event `self.OnInteract`
  (params (InteractingPlayer :type "Character Object Reference"))
  (bind _bp_electricitylight (`self.BP_ElectricityLight`))
  (if (`/Game/Blueprints/Actors/ElectricityBoxAndTrigger/BP_ElectricitySwitch.hasElectricity?` (`self.BP_ElectricitySwitch`))
    (if (`/Game/Blueprints/Actors/Lights/ElectricLights/BP_ElectricityLight.isLightOn?` (`self.BP_ElectricityLight`))
      (`/Game/Blueprints/Actors/Lights/ElectricLights/BP_ElectricityLight.TurnOffLight` _bp_electricitylight)
      (else
        (`/Game/Blueprints/Actors/Lights/ElectricLights/BP_ElectricityLight.TurnOnLight` _bp_electricitylight)))
    (else
      (`KismetSystemLibrary.PrintString` (`self.No Electricity Message`)))))

(event `self.ReceiveTick`
  (params (DeltaSeconds :type "Float (single-precision)"))
  (if (not (`/Game/Blueprints/Actors/ElectricityBoxAndTrigger/BP_ElectricitySwitch.hasElectricity?` (`self.BP_ElectricitySwitch`)))
    (`/Game/Blueprints/Actors/Lights/ElectricLights/BP_ElectricityLight.TurnOffLight` (`self.BP_ElectricityLight`))))

(fn `IsInteractable`
  (returns (Interactable :type Boolean))
  (return true))

(fn `UserConstructionScript`)