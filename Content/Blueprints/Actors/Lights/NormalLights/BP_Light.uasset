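; BP_Light is a light actor with an on/off state and configurable intensity, radius and color.
; Its construction script applies the IsLightOn state and pushes those settings to the LightSource component.
; TurnOnLight and TurnOffLight update the flag and toggle the component's visibility without propagating to children.
; The event graph has no active logic.
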(fn `TurnOffLight`
  (set `self.isLightOn?` false)
  (`SceneComponent.SetVisibility` (`self.LightSource`) false false))

(fn `TurnOnLight`
  (set `self.isLightOn?` true)
  (`SceneComponent.SetVisibility` (`self.LightSource`) true false))

(fn `UserConstructionScript`
  (bind _lightsource (`self.LightSource`))
  (if (`self.isLightOn?`)
    (`self.TurnOnLight`)
    (else
      (`self.TurnOffLight`)))
  (`LightComponent.SetIntensity` _lightsource (`self.LightIntensity`))
  (`LocalLightComponent.SetAttenuationRadius` _lightsource (`self.LightRadius`))
  (`LightComponent.SetLightColor` _lightsource (`self.LightColor`) true))