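; BP_WoodenSign is a sign actor that shows configurable text through its text component.
; The construction script applies the DisplayedText string and FontSize, then shifts the text by TextLocation as a world-space offset.
; BeginPlay repeats the same three calls, so the additive offset is applied again at runtime on top of the construction-time placement.
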(event `self.ReceiveBeginPlay`
  (bind _textcomponent (`self.TextComponent`))
  (`TextRenderComponent.K2_SetText` _textcomponent (`KismetTextLibrary.Conv_StringToText` (`self.DisplayedText`)))
  (`TextRenderComponent.SetWorldSize` _textcomponent (`self.Font Size`))
  (`SceneComponent.K2_AddWorldOffset` _textcomponent (`self.Text Location`) false false))

(fn `UserConstructionScript`
  (bind _textcomponent (`self.TextComponent`))
  (`TextRenderComponent.K2_SetText` _textcomponent (`KismetTextLibrary.Conv_StringToText` (`self.DisplayedText`)))
  (`TextRenderComponent.SetWorldSize` _textcomponent (`self.Font Size`))
  (`SceneComponent.K2_AddWorldOffset` _textcomponent (`self.Text Location`) false false))