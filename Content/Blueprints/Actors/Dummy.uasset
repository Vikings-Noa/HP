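; Dummy is a damageable target actor that shows its health as floating text and a health bar.
; A DecreaseValue event lowers the integer HP by a fixed step and refreshes the text.
; Each tick destroys the actor at zero HP or recolours the text through warning thresholds.
; Tick also pushes health into the WB_ZombieHealth widget's bar and rotates it to face the player camera.
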(event `self.ReceiveBeginPlay`
  (`TextRenderComponent.K2_SetText` (`self.Text renderer`) (`KismetTextLibrary.Conv_IntToText` (`self.HP(Int)`))))

(event `Decrease Value`
  (bind _output_get (set `self.HP(Int)` (- (`self.HP(Int)`) 5)))
  (`TextRenderComponent.K2_SetText` (`self.Text renderer`) (`KismetTextLibrary.Conv_IntToText` _output_get))
  (set `self.Health` (`KismetMathLibrary.Conv_IntToDouble` _output_get)))

(event `self.ReceiveTick`
  (params (DeltaSeconds :type "Float (single-precision)"))
  (bind _healthbarwidget (`self.HealthBarWidget`))
  (`|ExecutionSequence`
    (:`then_0`
      (if (<= (`self.HP(Int)`) 0)
        (`self.K2_DestroyActor`)
        (else
          (`|ExecutionSequence`
            (:`then_0`
              (if (<= (`self.HP(Int)`) 50)
                (`TextRenderComponent.SetTextRenderColor` (`self.Text renderer`) (`self.Yellow color`))))
            (:`then_1`
              (if (<= (`self.HP(Int)`) 25)
                (`TextRenderComponent.SetTextRenderColor` (`self.Text renderer`) (`self.Orange color`))))
            (:`then_2`
              (if (<= (`self.HP(Int)`) 15)
                (`TextRenderComponent.SetTextRenderColor` (`self.Text renderer`) (`self.Red color`))))))))
    (:`then_1`
      (`/Engine/EditorBlueprintResources/StandardMacros.IsValid` (`self.HealthBarWidget`)
        (:`Is Valid`
          (bind _aswb_zombie_health (cast `/Game/Blueprints/Widgets/WB_ZombieHealth` (`WidgetComponent.GetWidget` (`self.HealthBarWidget`))))
          (`ProgressBar.SetPercent` (`/Game/Blueprints/Widgets/WB_ZombieHealth.HealthBar` _aswb_zombie_health) (/ (`self.Health`) 100.0))
          (`SceneComponent.K2_SetWorldRotation` _healthbarwidget (`KismetMathLibrary.FindLookAtRotation` (`SceneComponent.K2_GetComponentLocation` _healthbarwidget) (`SceneComponent.K2_GetComponentLocation` (`PlayerCameraManager.TransformComponent` (`GameplayStatics.GetPlayerCameraManager` 0)))) false false))))))

(fn `UserConstructionScript`)