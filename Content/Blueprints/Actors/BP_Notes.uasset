(event `self.Box Collision.OnComponentEndOverlap`
  (params (OverlappedComponent :type "PrimitiveComponent Object Reference") (OtherActor :type "Actor Object Reference") (OtherComp :type "PrimitiveComponent Object Reference") (OtherBodyIndex :type Integer))
  (`/Game/Characters/Player/HP_Character.HideNote` (`self.Character Reference`)))

(event `/Game/Blueprints/Interfaces/BPI_Interact.OnInteract`
  (params (InteractingPlayer :type "Character Object Reference"))
  (if (`/Game/Characters/Player/HP_Character.NoteOnScreen?` (`self.Character Reference`))
    (set `/Game/Characters/Player/HP_Character.Note` (`self.NoteDescription`) (`self.Character Reference`))
    (set `/Game/Characters/Player/HP_Character.NoteOnScreen?` true (`self.Character Reference`))
    (`Widget.SetVisibility` (`/Game/UI/WB_MasterUI.WB_Note` (`/Game/Characters/Player/HP_Character.MasterUI Ref` (`self.Character Reference`))) "Visible")
    (`Widget.SetVisibility` (`/Game/UI/WB_MasterUI.WB_TAB` (`/Game/Characters/Player/HP_Character.MasterUI Ref` (`self.Character Reference`))) "Visible")
    (else
      (set `/Game/Characters/Player/HP_Character.Note` (`self.NoteDescription`) (`self.Character Reference`))
      (set `/Game/Characters/Player/HP_Character.NoteOnScreen?` true (`self.Character Reference`))
      (`GameplayStatics.PlaySound2D` "/Game/Audio/NotePickUp_Cue.NotePickUp_Cue" 1.0 1.0 0.0 null null)
      (`Widget.SetVisibility` (`/Game/UI/WB_MasterUI.WB_Note` (`/Game/Characters/Player/HP_Character.MasterUI Ref` (`self.Character Reference`))) "Visible")
      (`Widget.SetVisibility` (`/Game/UI/WB_MasterUI.WB_TAB` (`/Game/Characters/Player/HP_Character.MasterUI Ref` (`self.Character Reference`))) "Visible"))))

(fn `IsInteractable`
  (returns (Interactable :type Boolean))
  (return true))

(fn `UserConstructionScript`
  (`parent.UserConstructionScript`))