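; BP_TrapDoorButton is an always-interactable button that opens and closes a linked BPTrapDoorWithButton trapdoor.
; Interacting is ignored while the trapdoor animates; otherwise it flips the door's closed state and plays or reverses a timeline.
; The timeline alpha drives a roll rotation on the trapdoor's Pivot and clears the animating flag when finished.
; Both state flags live on the trapdoor rather than the button.
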(event `self.OnInteract`
  (params (InteractingPlayer :type "Character Object Reference"))
  (bind _bp_trapdoorwithbutton (`self.BP_TrapDoorWithButton`))
  (if (`/Game/Blueprints/Actors/Doors/BP_TrapDoorWIthButton.isTrapAnimating?` (`self.BP_TrapDoorWithButton`))
    _
    (elif (`/Game/Blueprints/Actors/Doors/BP_TrapDoorWIthButton.isTrapClosed?` (`self.BP_TrapDoorWithButton`))
      (set `/Game/Blueprints/Actors/Doors/BP_TrapDoorWIthButton.isTrapAnimating?` true _bp_trapdoorwithbutton)
      (set `/Game/Blueprints/Actors/Doors/BP_TrapDoorWIthButton.isTrapClosed?` false _bp_trapdoorwithbutton)
      (bind (_direction _alpha) (`Timeline|TrapdoorTimeline` :!label _label)
        (:`Update`
          (`SceneComponent.K2_SetRelativeRotation` (`/Game/Blueprints/Actors/Doors/BP_TrapDoorWIthButton.Pivot` (`self.BP_TrapDoorWithButton`)) (`KismetMathLibrary.MakeRotator` (`KismetMathLibrary.Lerp` 0.0 -120.0 _alpha)) false false))
        (:`Finished`
          (set `/Game/Blueprints/Actors/Doors/BP_TrapDoorWIthButton.isTrapAnimating?` false (`self.BP_TrapDoorWithButton`))))
      (else
        (set `/Game/Blueprints/Actors/Doors/BP_TrapDoorWIthButton.isTrapAnimating?` true _bp_trapdoorwithbutton)
        (set `/Game/Blueprints/Actors/Doors/BP_TrapDoorWIthButton.isTrapClosed?` true _bp_trapdoorwithbutton)
        (goto _label :!via `Reverse`)))))

(fn `IsInteractable`
  (returns (Interactable :type Boolean))
  (return true))

(fn `UserConstructionScript`)