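; BP_Doors is an interactable door actor that swings open and closed when the player interacts with it.
; OnInteract toggles the closed state, plays a 2D opening or closing sound, and plays or reverses the OpenDoor timeline.
; The timeline alpha lerps the Pivot's relative yaw through a quarter turn.
; An IsDoorAnimating flag ignores further interaction until the timeline finishes.
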(event `/Game/Blueprints/Interfaces/BPI_Interact.OnInteract`
  (params (InteractingPlayer :type "Character Object Reference"))
  (if (`self.IsDoorAnimating?`)
    _
    (elif (`self.IsDoorClosed`)
      (set `self.IsDoorAnimating?` true)
      (set `self.IsDoorClosed` false)
      (`GameplayStatics.PlaySound2D` "/Game/Audio/DoorOpeningSound.DoorOpeningSound" 1.0 1.0 0.0 null null)
      (bind (_direction _alpha) (`Timeline|OpenDoor` :!label _label)
        (:`Update`
          (`SceneComponent.K2_SetRelativeRotation` (`self.Pivot`) (`KismetMathLibrary.MakeRotator` 0.0 0.0 (`KismetMathLibrary.Lerp` 0.0 90.0 _alpha)) false false))
        (:`Finished`
          (set `self.IsDoorAnimating?` false)))
      (else
        (set `self.IsDoorAnimating?` true)
        (set `self.IsDoorClosed` true)
        (`GameplayStatics.PlaySound2D` "/Game/Audio/DoorClosingSound.DoorClosingSound" 1.0 1.0 0.0 null null)
        (goto _label :!via `Reverse`)))))

(fn `IsInteractable`
  (returns (Interactable :type Boolean))
  (return true))

(fn `UserConstructionScript`
  (`parent.UserConstructionScript`))