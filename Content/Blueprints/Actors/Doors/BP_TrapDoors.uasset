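; BP_TrapDoors is an interactable trap door that toggles open and closed when the player interacts with it.
; OnInteract plays or reverses the OpeningTrap timeline, which lerps the Pivot component's relative roll to swing the door 120 degrees.
; An IsTrapAnimating flag ignores input during the swing and clears when the timeline finishes, while IsTrapClosed tracks the current state.
; IsInteractable always returns true.
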(event `self.OnInteract`
  (params (InteractingPlayer :type "Character Object Reference"))
  (if (`self.isTrapAnimating?`)
    _
    (elif (`self.isTrapClosed?`)
      (set `self.isTrapAnimating?` true)
      (set `self.isTrapClosed?` false)
      (bind (_direction _alpha) (`Timeline|OpeningTrap` :!label _label)
        (:`Update`
          (`SceneComponent.K2_SetRelativeRotation` (`self.Pivot`) (`KismetMathLibrary.MakeRotator` (`KismetMathLibrary.Lerp` 0.0 -120.0 _alpha)) false false))
        (:`Finished`
          (set `self.isTrapAnimating?` false)))
      (else
        (set `self.isTrapAnimating?` true)
        (set `self.isTrapClosed?` true)
        (goto _label :!via `Reverse`)))))

(fn `IsInteractable`
  (returns (Interactable :type Boolean))
  (return true))

(fn `UserConstructionScript`)