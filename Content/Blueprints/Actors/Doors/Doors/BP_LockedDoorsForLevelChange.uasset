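; A key-locked interactable door that leads the player to another level.
; Interacting without the key plays a locked sound and prints the door name; with it, the first use unlocks after a short delay, then a timeline swings the pivot open or closed.
; Once unlocked, HP_Character entering the trigger spawns a fade widget with a shutter sound, then opens the named level after a delay.
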(event `self.Pick Up Key`
  (set `self.HasKey?` true)
  (`KismetSystemLibrary.PrintString` (`self.KeyName`) true true (struct :`R` 1.0 :`G` 0.327564 :`A` 1.0) 5.0))

(event `self.OnInteract`
  (params (InteractingPlayer :type "Character Object Reference"))
  (if (`self.HasKey?`)
    (if (`self.IsDoorAnimating?`)
      _
      (elif (`self.HasBeenUnlocked`)
        (if (`self.IsDoorClosed`)
          (set `self.IsDoorAnimating?` true)
          (set `self.IsDoorClosed` false)
          (`GameplayStatics.PlaySound2D` "/Game/Audio/DoorOpeningSound.DoorOpeningSound" 1.0 1.0 0.0 null null :!label _label)
          (bind (_direction _alpha) (`Timeline|OpenDoor` :!label _label_2)
            (:`Update`
              (`SceneComponent.K2_SetRelativeRotation` (`self.Pivot`) (`KismetMathLibrary.MakeRotator` 0.0 0.0 (`KismetMathLibrary.Lerp` 0.0 100.0 _alpha)) false false))
            (:`Finished`
              (set `self.IsDoorAnimating?` false)))
          (else
            (set `self.IsDoorAnimating?` true)
            (set `self.IsDoorClosed` true)
            (`GameplayStatics.PlaySound2D` "/Game/Audio/DoorClosingSound.DoorClosingSound" 1.0 1.0 0.0 null null)
            (goto _label_2 :!via `Reverse`)))
        (else
          (`GameplayStatics.PlaySound2D` "/Game/Audio/DoorUnlockSound.DoorUnlockSound" 1.0 1.0 0.0 null null)
          (`KismetSystemLibrary.Delay` 0.8)
          (set `self.HasBeenUnlocked` true)
          (if (`self.IsDoorClosed`)
            (set `self.IsDoorAnimating?` true)
            (set `self.IsDoorClosed` false)
            (goto _label)))))
    (else
      (`GameplayStatics.PlaySound2D` "/Game/Audio/LockeedDoorSoubd.LockeedDoorSoubd" 1.0 1.0 0.0 null null)
      (`KismetSystemLibrary.PrintString` (`self.DoorName`) true true (struct :`R` 1.0 :`A` 1.0) 5.0))))

(event `self.Trigger.OnComponentBeginOverlap`
  (params (OverlappedComponent :type "PrimitiveComponent Object Reference") (OtherActor :type "Actor Object Reference") (OtherComp :type "PrimitiveComponent Object Reference") (OtherBodyIndex :type Integer) (bFromSweep :type Boolean) (SweepResult :type "HitResult Structure (by ref)"))
  (cast `/Game/Characters/Player/HP_Character` OtherActor)
  (if (`self.HasBeenUnlocked`)
    (`GameplayStatics.PlaySound2D` "/Engine/VREditor/Sounds/UI/Camera_Shutter.Camera_Shutter" 1.0 1.0 0.0 null null)
    (bind _returnvalue (`|CreateWidget` "/Game/UI/WB_ChangingLevel.WB_ChangingLevel_C"))
    (`UserWidget.AddToViewport` _returnvalue 0)
    (`/Game/UI/WB_ChangingLevel.Fade` _returnvalue)
    (`KismetSystemLibrary.Delay` 3.333)
    (`GameplayStatics.OpenLevel` (`self.Level Name`))))

(fn `IsInteractable`
  (returns (Interactable :type Boolean))
  (return true))

(fn `UserConstructionScript`
  (`parent.UserConstructionScript`))